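; Game mode that opens the main menu when play begins and shows the mouse cursor.
; BeginPlay creates the main menu and the in-game HUD, cross-links them with the game mode, and adds only the menu to the viewport.
; Logic for a pausing end menu and an input-driven pause menu exists but is disconnected, so Tick does nothing.
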(event `self.ReceiveBeginPlay`
  (bind _startmenuhud (`self.StartMenuHUD`))
  ;[1 1 1] start menu
  (bind _returnvalue (`|CreateWidget` "/Game/Blueprints/BP_MainMenu.BP_MainMenu_C"))
  (bind _output_get (set `self.StartMenuHUD` _returnvalue))
  ;[1 1 1] set game mode
  (set `/Game/Blueprints/BP_MainMenu.GameMode` self _output_get)
  (`UserWidget.AddToViewport` _output_get 0)
  ;[1 1 1] set in game hud
  (bind _returnvalue_2 (`|CreateWidget` "/Game/Blueprints/BP_MyHUD.BP_MyHUD_C"))
  (set `/Game/Blueprints/BP_MainMenu.GameHUD` _returnvalue_2 _startmenuhud)
  (set `/Game/Blueprints/BP_MyHUD.MyGameMode` self (`/Game/Blueprints/BP_MainMenu.GameHUD` _startmenuhud))
  (set `PlayerController.bShowMouseCursor` true (`GameplayStatics.GetPlayerController` 0))
  (`self.SetActorTickEnabled` true))

(event `self.ReceiveTick`
  (params (DeltaSeconds :type "Float (single-precision)")))

(fn `UserConstructionScript`)